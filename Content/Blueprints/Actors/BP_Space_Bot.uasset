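; Flying companion bot that follows the player and, if allowed, occasionally turns angry to shove them.
; Looping timers face the mesh at the player, pick a random point above them when too far away, and run front and vertical avoidance traces.
; Tick applies physics forces to steer and brake the sphere.
; Anger changes the emissive material, spawns Niagara and starts a timed push that launches the player on overlap.
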(event `Orient Bot`
  ; LOOK AT PLAYER
  (`SceneComponent.K2_SetRelativeRotation` (`self.SM_Space_Bot`) (`KismetMathLibrary.MakeRotator` (.roll (`KismetMathLibrary.FindLookAtRotation` (`SceneComponent.K2_GetComponentLocation` (`self.SM_Space_Bot`)) (`self.K2_GetActorLocation` (`self.Player`)))) (.pitch (`KismetMathLibrary.FindLookAtRotation` (`SceneComponent.K2_GetComponentLocation` (`self.SM_Space_Bot`)) (`self.K2_GetActorLocation` (`self.Player`)))) (- (.yaw (`KismetMathLibrary.FindLookAtRotation` (`SceneComponent.K2_GetComponentLocation` (`self.SM_Space_Bot`)) (`self.K2_GetActorLocation` (`self.Player`)))) 90.0)) false false))

(event `self.ReceiveBeginPlay`
  ; set dyn material for the light
  (bind _returnvalue (`PrimitiveComponent.CreateDynamicMaterialInstance` (`self.SM_Space_Bot`) 0 null "None"))
  (set `self.DynMaterial` _returnvalue)
  (`SceneComponent.SetAbsolute` (`self.SM_Space_Bot`) false true false)
  ; set the player if valid
  (bind _returnvalue_2 (`GameplayStatics.GetActorOfClass` "/Game/Blueprints/Actors/Pawn/BP_ThirdPersonCharacter.BP_ThirdPersonCharacter_C"))
  (set `self.Player` _returnvalue_2)
  (`/Engine/EditorBlueprintResources/StandardMacros.IsValid` (`self.Player`)
    (:`Is Valid`
      ; Deplacement
      (`KismetSystemLibrary.K2_SetTimerDelegate` (delegate `Check On Player`) 1.0 true)
      ; Look at player
      (`KismetSystemLibrary.K2_SetTimerDelegate` (delegate `Orient Bot`) 0.01 true)
      ; Avoidance
      (`KismetSystemLibrary.K2_SetTimerDelegate` (delegate `AvoidabceSystem`) 0.2 true)
      (`self.CanPush`
        (:`then`
          (`KismetSystemLibrary.K2_SetTimerDelegate` (delegate `Angry ?`) 5.0 true))
        (:`else`)))))

(event `Angry ?`
  (bind _dynmaterial (`self.DynMaterial`))
  (bind _dynmaterial_2 (`self.DynMaterial`))
  (`self.AsANewLocation`
    (:`then`)
    (:`else`
      (`self.Is Pushing`
        (:`then`)
        (:`else`
          (if (> (`KismetMathLibrary.RandomFloatInRange` 0.0 1.0) 0.9)
            (`MaterialInstanceDynamic.SetVectorParameterValue` _dynmaterial_2 "Emissive_Color" (struct :`R` 1.0 :`G` 0.01843 :`B` 0.000363 :`A` 1.0))
            (`MaterialInstanceDynamic.SetScalarParameterValue` _dynmaterial_2 "Emissive_Strenght" 50.0)
            (`NiagaraFunctionLibrary.SpawnSystemAtLocation` "/Game/Trash/NewNiagaraSystem.NewNiagaraSystem" (`SceneComponent.K2_GetComponentLocation` (`self.Sphere`)))
            (`KismetSystemLibrary.Delay` 1.3)
            (set `self.Is Pushing` true)
            (`KismetSystemLibrary.K2_SetTimerDelegate` (delegate `StopPushing`) 6.0)
            (`KismetSystemLibrary.PrintString` "grrrrrrrrrrrrrrr")
            (else
              (`MaterialInstanceDynamic.SetVectorParameterValue` _dynmaterial "Emissive_Color" (struct :`R` 0.991102 :`G` 0.074214 :`B` 1.0 :`A` 1.0))
              (`MaterialInstanceDynamic.SetScalarParameterValue` _dynmaterial "Emissive_Strenght" 1.0)
              (set `self.Is Pushing` false))))))))

(event `StopPushing`
  (bind _dynmaterial (`self.DynMaterial`))
  (`MaterialInstanceDynamic.SetVectorParameterValue` _dynmaterial "Emissive_Color" (struct :`R` 0.991102 :`G` 0.074214 :`B` 1.0 :`A` 1.0))
  (`MaterialInstanceDynamic.SetScalarParameterValue` _dynmaterial "Emissive_Strenght" 1.0)
  (set `self.Is Pushing` false)
  (`self.Get New Point`))

(event `Check On Player`
  ;[0.15 0.15 0.15 0.5 50] GO AT LOCATION
  ;; bot to player distance
  (if (> (`KismetMathLibrary.Vector_Distance` (`SceneComponent.K2_GetComponentLocation` (`self.Sphere`)) (`self.K2_GetActorLocation` (`self.Player`))) (`self.MAXDistanceFromPlayer`))
    (set `self.AsANewLocation` true)
    (`self.CanGetNewLocation`
      (:`then`
        ;; Get Random Point in Radius around player (top half of a sphere)
        (set `self.CanGetNewLocation` false :!label _label)
        (set `self.TargetPoint` (+ (`self.K2_GetActorLocation` (`self.Player`)) (* (`KismetMathLibrary.MakeVector` (.x (`KismetMathLibrary.RandomUnitVector`)) (.y (`KismetMathLibrary.RandomUnitVector`)) (`KismetMathLibrary.FClamp` (`KismetMathLibrary.Abs` (.z (`KismetMathLibrary.RandomUnitVector`))) 0.1 0.5)) (`KismetMathLibrary.RandomFloatInRange` (`self.Min range from player`) (`self.Max range from player`))))))
      (:`else`))
    (else
      (set `self.AsANewLocation` false))))

(event `Get New Point`
  ;[0.15 0.15 0.15 0.5 50] GO AT LOCATION
  (goto _label))

(event `self.ReceiveTick`
  (params (DeltaSeconds :type "Float (single-precision)"))
  (bind _returnvalue (`KismetMathLibrary.Vector_Distance` (`SceneComponent.K2_GetComponentLocation` (`self.Sphere`)) (`self.TargetPoint`)))
  ;[0.15 0.15 0.15 0.5 100] moving system
  (`self.Is Pushing`
    (:`then`
      (`KismetSystemLibrary.Delay` (`self.DelayInpulsepushSpeed`))
      (`PrimitiveComponent.AddForce` (`self.Sphere`) (* (`KismetMathLibrary.Normal` (- (`SceneComponent.K2_GetComponentLocation` (`self.Sphere`)) (`self.K2_GetActorLocation` (`self.Player`)))) (`self.PushSpeed`)) "None" true))
    (:`else`
      (`self.AsANewLocation`
        (:`then`
          (if (stale `AvoidabceSystem` _returnvalue_3) :!label _label_2
            ;; X avoidance
            (`self.Z_Priority`
              (:`then`)
              (:`else`
                (`PrimitiveComponent.AddForce` (`self.Sphere`) (* (`.Normal` (`GameplayStatics.BreakHitResult` (stale `AvoidabceSystem` _outhit))) (750.0 0.0 -1500.0)) "None" true)
                (`PrimitiveComponent.AddForce` (`self.Sphere`) (0.0 1250.0 0.0) "None" true)))
            (else
              (`self.Z_Priority`
                (:`then`)
                (:`else`
                  (if (<= _returnvalue (`self.SlowDownDistance`))
                    ;; MAKE THE DRONE MOVE
                    (bind _returnvalue_2 (`PrimitiveComponent.GetPhysicsLinearVelocity` (`self.Sphere`) "None"))
                    (bind _returnvalue_3 (`KismetMathLibrary.VSize` _returnvalue_2))
                    (`PrimitiveComponent.AddForce` (`self.Sphere`) (* _returnvalue_2 (* _returnvalue_3 (* (`self.BreakStrengh`) -1.0))) "None" true)
                    (`KismetSystemLibrary.PrintString` (`KismetStringLibrary.Conv_DoubleToString` _returnvalue_3) true true (struct :`G` 0.66 :`B` 1.0 :`A` 1.0) 0.0 "speed")
                    (if (<= _returnvalue_3 200.0)
                      (set `self.CanGetNewLocation` true)
                      (`KismetSystemLibrary.PrintString` "arrived" true true (struct :`R` 0.21611 :`G` 1.0 :`A` 1.0) 1000.0 "speed"))
                    (else
                      ;; MAKE THE DRONE MOVE
                      (`PrimitiveComponent.AddForce` (`self.Sphere`) (* (`KismetMathLibrary.Normal` (- (`self.TargetPoint`) (`SceneComponent.K2_GetComponentLocation` (`self.Sphere`)))) (`KismetMathLibrary.FClamp` _returnvalue -200.0 200.0)) "None" true))))))))
        (:`else`)))))

(event `AvoidabceSystem`
  (bind _arrowx (`self.ArrowX`))
  (bind _arrowz (`self.ArrowZ`))
  (bind _returnvalue (`SceneComponent.K2_GetComponentLocation` _arrowx))
  (bind _returnvalue_2 (`SceneComponent.K2_GetComponentLocation` _arrowz))
  ;[0.15 0.15 0.15 0.5 100] moving system
  (`self.AsANewLocation`
    (:`then`
      (`|ExecutionSequence`
        (:`then_0`
          ;; X avoidance
          (bind (_outhit _returnvalue_3) (`KismetSystemLibrary.LineTraceSingle` :`Start` _returnvalue :`End` (+ _returnvalue (* (`KismetMathLibrary.GetForwardVector` (`SceneComponent.K2_GetComponentRotation` _arrowx)) 1000.0)) :`TraceChannel` "TraceTypeQuery1" :`bTraceComplex` true :`TraceColor` (struct :`R` 1.0 :`B` 0.035999 :`A` 1.0) :`TraceHitColor` (struct :`R` 1.0 :`G` 1.0 :`B` 1.0 :`A` 1.0) :`DrawTime` 0.2))
          (goto _label_2))
        (:`then_1`
          ;; Comment
          (bind (_outhit_2 _returnvalue_4) (`KismetSystemLibrary.LineTraceSingle` :`Start` _returnvalue_2 :`End` (+ _returnvalue_2 (* (`KismetMathLibrary.GetForwardVector` (`SceneComponent.K2_GetComponentRotation` _arrowz)) 350.0)) :`TraceChannel` "TraceTypeQuery1" :`bTraceComplex` true :`TraceColor` (struct :`G` 0.618129 :`B` 1.0 :`A` 1.0) :`TraceHitColor` (struct :`R` 1.0 :`G` 1.0 :`B` 1.0 :`A` 1.0) :`DrawTime` 0.2))
          (if _returnvalue_4
            (set `self.Z_Priority` true)
            (`PrimitiveComponent.AddForce` (`self.Sphere`) (* (`.ImpactPoint` (`GameplayStatics.BreakHitResult` _outhit_2)) (-1000.0 0.0 500.0)) "None" false)
            (else
              (set `self.Z_Priority` false))))))
    (:`else`)))

(event `self.Sphere.OnComponentBeginOverlap`
  (params (OverlappedComponent :type "PrimitiveComponent Object Reference") (OtherActor :type "Actor Object Reference") (OtherComp :type "PrimitiveComponent Object Reference") (OtherBodyIndex :type Integer) (bFromSweep :type Boolean) (SweepResult :type "HitResult Structure (by ref)"))
  (bind (_returnvalue_x _returnvalue_y) (`KismetMathLibrary.BreakVector` (* (`KismetMathLibrary.Normal` (- (`SceneComponent.K2_GetComponentLocation` (`self.Sphere`)) (`self.K2_GetActorLocation` (`self.Player`)))) -3000.0)))
  (`self.Is Pushing`
    (:`then`
      (cast `CapsuleComponent` OtherComp)
      (bind _asbp_third_person_character (cast `/Game/Blueprints/Actors/Pawn/BP_ThirdPersonCharacter` OtherActor))
      (`KismetSystemLibrary.PrintString` "touched")
      (`Character.LaunchCharacter` _asbp_third_person_character (`KismetMathLibrary.MakeVector` _returnvalue_x _returnvalue_y 200.0) true true)
      (`self.StopPushing`))
    (:`else`)))

(fn `UserConstructionScript`)