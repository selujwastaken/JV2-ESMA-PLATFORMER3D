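; BP_MasterCube is a physics cube that previews its launch trajectory, records distance moved and can respawn at its start point.
; PredictPath estimates radial-force impulse with falloff, feeds projectile prediction into a spline and enables Tick to attach a Niagara ribbon.
; A looping timer uses velocity thresholds to mark start and rest positions, adding their distance to BP_GameInstance.
; RESPAWN scales the cube, spawns a destroy effect, then replaces itself with an animated new instance.
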(event `RespawnAnim`
  ; play anim
  (bind (_direction _newtrack_0) (`Timeline|Timeline_0`)
    (:`Update`
      (`SceneComponent.SetRelativeScale3D` (`self.Box_TOP`) (`KismetMathLibrary.Conv_DoubleToVector` _newtrack_0))
      (`SceneComponent.SetRelativeScale3D` (`self.Box_BODY`) (`KismetMathLibrary.Conv_DoubleToVector` _newtrack_0)))))

(event `RESPAWN`
  (bind _box_top (`self.Box_TOP`))
  ;[0.15 0.15 0.15 0.5 50] RESPAWN CUBE
  (bind (_direction _newtrack_0) (`Timeline|Timeline`)
    (:`Update`
      (`SceneComponent.SetRelativeScale3D` _box_top (`KismetMathLibrary.Conv_DoubleToVector` _newtrack_0))
      (`SceneComponent.SetRelativeScale3D` (`self.Box_BODY`) (`KismetMathLibrary.Conv_DoubleToVector` _newtrack_0)))
    (:`Finished`
      (`NiagaraFunctionLibrary.SpawnSystemAtLocation` "/Game/Graphics/Niagara_Systems/NS_CubeDestroy.NS_CubeDestroy" (`SceneComponent.K2_GetComponentLocation` _box_top) (`SceneComponent.K2_GetComponentRotation` _box_top))
      (`self.K2_DestroyActor`)
      (bind _returnvalue (`|SpawnActorFromClass` "BP_MasterCube_C" (`KismetMathLibrary.MakeTransform` (`self.Spawned_Location`)) "Undefined" "MultiplyWithRoot" null null))
      (`self.RespawnAnim` _returnvalue))))

(event `self.ReceiveBeginPlay`
  ;[0.15 0.15 0.15 0.5 50] BEGIN PLAY
  (`KismetSystemLibrary.K2_SetTimerDelegate` (delegate `Get Positions`) 0.1 true)
  (set `self.Spawned_Location` (`self.K2_GetActorLocation`)))

(event `Get Positions`
  ;[0.15 0.15 0.15 0.5 50] GET HOW FAR HE DID TRAVEL
  (`self.AS_Set_Pos_A`
    (:`then`
      (`self.AS_Set_Pos_B`
        (:`then`
          ;; GET DISTANCE AND STORE IT
          (bind _asbp_game_instance (cast `/Game/Blueprints/BP_GameInstance` (`GameplayStatics.GetGameInstance`)))
          (set `/Game/Blueprints/BP_GameInstance.CubeDistanceParcourue` (+ (`/Game/Blueprints/BP_GameInstance.CubeDistanceParcourue` _asbp_game_instance) (`KismetMathLibrary.Vector_Distance` (`self.Location_A`) (`self.Location_B`))) _asbp_game_instance)
          (set `self.AS_Set_Pos_A` false)
          (set `self.AS_Set_Pos_B` false))
        (:`else`
          ;; GET VELOCITY AND MARK POS B
          (bind _returnvalue (`PrimitiveComponent.GetPhysicsLinearVelocity` (`self.Box_TOP`) "None"))
          (if (< (`KismetMathLibrary.VSize` _returnvalue) 3.0)
            (set `self.AS_Set_Pos_B` true)
            (set `self.Location_B` (`SceneComponent.K2_GetComponentLocation` (`self.Box_TOP`)))))))
    (:`else`
      ;; GET VELOCITY AND MARK POS A
      (bind _returnvalue_2 (`PrimitiveComponent.GetPhysicsLinearVelocity` (`self.Box_TOP`) "None"))
      (if (> (`KismetMathLibrary.VSize` _returnvalue_2) 10.0)
        (set `self.AS_Set_Pos_A` true)
        (set `self.Location_A` (`SceneComponent.K2_GetComponentLocation` (`self.Box_TOP`)))))))

(event `self.ReceiveTick`
  (params (DeltaSeconds :type "Float (single-precision)"))
  (`self.Is_Simulated`
    (:`then`
      (`self.AS_Spawned_Ribbon`
        (:`then`)
        (:`else`
          (set `self.AS_Spawned_Ribbon` true)
          (bind _returnvalue (`NiagaraFunctionLibrary.SpawnSystemAttached` "/Game/Graphics/Niagara_Systems/NS_RibbonTrajectory.NS_RibbonTrajectory" (`self.TrajectorySpline`) "None" (`SceneComponent.K2_GetComponentLocation` (`self.TrajectorySpline`)) (struct) "KeepRelativeOffset"))
          (bind _output_get (set `self.NS_Ribbon` _returnvalue))
          (`NiagaraComponent.SetVariableVec3` _output_get "User.HeadPosition" (0.0 0.0 0.0)))))
    (:`else`)))

(event `RESET`
  (bind _trajectoryspline (`self.TrajectorySpline`))
  (bind _ns_ribbon (`self.NS_Ribbon`))
  ;[0.15 0.15 0.15 0.5 50] RESET PREDICTION
  (set `self.Is_Simulated` false)
  (`/Engine/EditorBlueprintResources/StandardMacros.IsValid` _trajectoryspline
    (:`Is Valid`
      (`SplineComponent.ClearSplinePoints` _trajectoryspline true))
    (:`Is Not Valid`
      _))
  (`self.SetActorTickEnabled` false)
  (`/Engine/EditorBlueprintResources/StandardMacros.IsValid` _ns_ribbon
    (:`Is Valid`
      (`ActorComponent.K2_DestroyComponent` _ns_ribbon)
      (set `self.AS_Spawned_Ribbon` false)
      (set `self.AS_Set_Pos_A` false)
      (set `self.AS_Set_Pos_B` false))))

(event `Predict Path`
  (params (ForceIntecity :type Integer) (RadialForce :type "RadialForceComponent Object Reference"))
  (bind _box_top (`self.Box_TOP`))
  (bind _radius (`RadialForceComponent.Radius` (`self.Radial Force`)))
  (bind _returnvalue (- (`self.Simulated_Position`) (`SceneComponent.K2_GetComponentLocation` (`self.Radial Force`))))
  ;[0.15 0.15 0.15 0.5 100] PREDICT
  ;; GET ALL INFORMATIONS OF CUBE
  (set `self.Force Intecity` ForceIntecity)
  (set `self.Radial Force` RadialForce)
  (set `self.Is_Simulated` true)
  (bind _returnvalue_2 (`PrimitiveComponent.GetPhysicsLinearVelocity` _box_top "None"))
  (set `self.Simulated_Position` (`SceneComponent.K2_GetComponentLocation` _box_top))
  ;; CALCULER LA VÉLOCITÉ INITIALE POUR LA PRÉDICTION
  (set `self.Simulated_Velocity` (+ (+ (/ (* (`KismetMathLibrary.Normal` _returnvalue) (* (`RadialForceComponent.ImpulseStrength` (`self.Radial Force`)) (- 1.0 (/ (`KismetMathLibrary.FClamp` (`KismetMathLibrary.VSize` _returnvalue) 0.0 _radius) _radius)))) (/ (100.0 100.0 100.0) (`PrimitiveComponent.GetMass` (`self.Box_TOP`)))) (`KismetMathLibrary.MakeVector` 0.0 0.0 (`KismetMathLibrary.Conv_IntToDouble` (`self.Force Intecity`)))) _returnvalue_2))
  ;; SIMULER LA TRAJECTOIRE (BOUCLE)
  (bind _predictresult (`GameplayStatics.Blueprint_PredictProjectilePath_Advanced` (make `PredictProjectilePathParams` (`self.Simulated_Position`) (+ (`self.Simulated_Velocity`) (* -980.0 (`self.Time_Step`))) true 0.0 5.0 true "ECC_WorldStatic" _ _ 20.0 0.0 "ForOneFrame" 0.0 true)))
  (`SplineComponent.ClearSplinePoints` (`self.TrajectorySpline`) true)
  (for _array_element (`.PathData` (break `PredictProjectilePathResult` _predictresult))
    (`SplineComponent.AddSplinePoint` (`self.TrajectorySpline`) (`.Location` (break `PredictProjectilePathPointData` _array_element)) "World" true)
    (`self.SetActorTickEnabled` true)))

(fn `UserConstructionScript`)