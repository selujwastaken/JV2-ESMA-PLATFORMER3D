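; BP_Door is a gate that opens once, either immediately or when the achieved total matches TotalToGet if NeedMultiple is valid.
; A timeline drives the gate by adding a Z offset on each update.
; If IsACheckPoint is valid, opening also sets the player's checkpoint to the Arrow location and calls GivePublic once.
; The construction script shows requirement text only for multiple-requirement doors.
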(event `Open`
  (params (`Total Achived` :type Integer))
  (`self.need Multiple ?`
    (:`then`
      (if (== `Total Achived` (`self.total to get`))
        (`/Engine/EditorBlueprintResources/StandardMacros.DoOnce` false :!label _label
          (:`Completed`
            (bind (_direction _newtrack_0) (`Timeline|door`)
              (:`Update`
                (`SceneComponent.K2_AddLocalOffset` (`self.SM_Gate`) (`KismetMathLibrary.MakeVector` 0.0 0.0 (* _newtrack_0 8.0)) false false)
                (`self.Is A CheckPoint`
                  (:`then`
                    (bind _asbp_third_person_character (cast `/Game/Blueprints/Actors/Pawn/BP_ThirdPersonCharacter` (`GameplayStatics.GetPlayerCharacter` 0)))
                    (set `/Game/Blueprints/Actors/Pawn/BP_ThirdPersonCharacter.CheckPoint` (`SceneComponent.K2_GetComponentLocation` (`self.Arrow`)) _asbp_third_person_character)
                    (`/Engine/EditorBlueprintResources/StandardMacros.DoOnce` false
                      (:`Completed`
                        (`/Game/Blueprints/Actors/Pawn/BP_ThirdPersonCharacter.Give Public` _asbp_third_person_character 10.0))))
                  (:`else`))))))))
    (:`else`
      (goto _label))))

(fn `UserConstructionScript`
  (bind _number_left (`self.NUMBER LEFT`))
  (`self.need Multiple ?`
    (:`then`
      (`SceneComponent.SetVisibility` _number_left true false)
      (`SceneComponent.SetVisibility` (`self.You Have`) true false)
      (`TextRenderComponent.K2_SetText` (`self.NUMBER LEFT`) (`KismetTextLibrary.Conv_StringToText` (`KismetStringLibrary.Concat_StrStr` "YOU NEED : " (`KismetStringLibrary.Conv_IntToString` (`self.total to get`)) " LEFT"))))
    (:`else`
      (`SceneComponent.SetVisibility` _number_left false false)
      (`SceneComponent.SetVisibility` (`self.You Have`) false false))))