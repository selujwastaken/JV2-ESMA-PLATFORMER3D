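; BP_Energy_Drink is a pickup actor that permanently boosts the player's stamina.
; It spins slowly by stepping its yaw every Tick, without scaling by delta time.
; When a BP_ThirdPersonCharacter's capsule overlaps its Sphere, it destroys itself, raises that character's max stamina, current stamina and stamina gain value, and calls GivePublic on it.
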(event `self.ReceiveTick`
  (params (DeltaSeconds :type "Float (single-precision)"))
  (bind (_returnvalue_roll _returnvalue_pitch _returnvalue_yaw) (`KismetMathLibrary.BreakRotator` (`self.K2_GetActorRotation`)))
  (`self.K2_SetActorRotation` (`KismetMathLibrary.MakeRotator` _returnvalue_roll _returnvalue_pitch (+ _returnvalue_yaw -0.8))))

(event `self.Sphere.OnComponentBeginOverlap`
  (params (OverlappedComponent :type "PrimitiveComponent Object Reference") (OtherActor :type "Actor Object Reference") (OtherComp :type "PrimitiveComponent Object Reference") (OtherBodyIndex :type Integer) (bFromSweep :type Boolean) (SweepResult :type "HitResult Structure (by ref)"))
  (cast `CapsuleComponent` OtherComp)
  (bind _asbp_third_person_character (cast `/Game/Blueprints/Actors/Pawn/BP_ThirdPersonCharacter` OtherActor))
  (`self.K2_DestroyActor`)
  (set `/Game/Blueprints/Actors/Pawn/BP_ThirdPersonCharacter.Stamina_Max` (+ (`/Game/Blueprints/Actors/Pawn/BP_ThirdPersonCharacter.Stamina_Max` _asbp_third_person_character) 25.0) _asbp_third_person_character)
  (set `/Game/Blueprints/Actors/Pawn/BP_ThirdPersonCharacter.Stamina` (+ (`/Game/Blueprints/Actors/Pawn/BP_ThirdPersonCharacter.Stamina` _asbp_third_person_character) 25.0) _asbp_third_person_character)
  (set `/Game/Blueprints/Actors/Pawn/BP_ThirdPersonCharacter.StaminaGainValue` (+ (`/Game/Blueprints/Actors/Pawn/BP_ThirdPersonCharacter.StaminaGainValue` _asbp_third_person_character) 0.1) _asbp_third_person_character)
  (`/Game/Blueprints/Actors/Pawn/BP_ThirdPersonCharacter.Give Public` _asbp_third_person_character 10.0))

(fn `UserConstructionScript`)