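; Interactable actor that shows a "PRESSE" prompt while the third-person character is inside its sphere, with an empty INTERACTION event as the interaction hook.
; Sphere overlaps toggle the prompt's visibility and set or clear the character's reference to this actor.
; A looping timer, rather than Tick, turns the prompt toward the follow camera, applying a yaw offset to the look-at rotation.
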(event `self.ReceiveBeginPlay`
  (bind _returnvalue (`GameplayStatics.GetActorOfClass` "/Game/Blueprints/Actors/Pawn/BP_ThirdPersonCharacter.BP_ThirdPersonCharacter_C"))
  (set `self.Character` _returnvalue)
  (`KismetSystemLibrary.K2_SetTimerDelegate` (delegate `TextLookAtPlayer`) 0.2 true))

(event `TextLookAtPlayer`
  (bind _character (`self.Character`))
  (`/Engine/EditorBlueprintResources/StandardMacros.IsValid` _character
    (:`Is Valid`
      (`SceneComponent.K2_SetRelativeRotation` (`self.PRESS E`) (`KismetMathLibrary.MakeRotator` (.roll (`KismetMathLibrary.FindLookAtRotation` (`self.K2_GetActorLocation`) (`SceneComponent.K2_GetComponentLocation` (`/Game/Blueprints/Actors/Pawn/BP_ThirdPersonCharacter.FollowCamera` _character)))) (.pitch (`KismetMathLibrary.FindLookAtRotation` (`self.K2_GetActorLocation`) (`SceneComponent.K2_GetComponentLocation` (`/Game/Blueprints/Actors/Pawn/BP_ThirdPersonCharacter.FollowCamera` _character)))) (+ (.yaw (`KismetMathLibrary.FindLookAtRotation` (`self.K2_GetActorLocation`) (`SceneComponent.K2_GetComponentLocation` (`/Game/Blueprints/Actors/Pawn/BP_ThirdPersonCharacter.FollowCamera` _character)))) -90.0)) false false))))

(event `self.Sphere.OnComponentBeginOverlap`
  (params (OverlappedComponent :type "PrimitiveComponent Object Reference") (OtherActor :type "Actor Object Reference") (OtherComp :type "PrimitiveComponent Object Reference") (OtherBodyIndex :type Integer) (bFromSweep :type Boolean) (SweepResult :type "HitResult Structure (by ref)"))
  (bind _asbp_third_person_character (cast `/Game/Blueprints/Actors/Pawn/BP_ThirdPersonCharacter` OtherActor))
  (`SceneComponent.SetVisibility` (`self.PRESS E`) true false)
  (set `/Game/Blueprints/Actors/Pawn/BP_ThirdPersonCharacter.BP_Interactable` self _asbp_third_person_character))

(event `self.Sphere.OnComponentEndOverlap`
  (params (OverlappedComponent :type "PrimitiveComponent Object Reference") (OtherActor :type "Actor Object Reference") (OtherComp :type "PrimitiveComponent Object Reference") (OtherBodyIndex :type Integer))
  (bind _asbp_third_person_character (cast `/Game/Blueprints/Actors/Pawn/BP_ThirdPersonCharacter` OtherActor))
  (`SceneComponent.SetVisibility` (`self.PRESS E`) false false)
  (set `/Game/Blueprints/Actors/Pawn/BP_ThirdPersonCharacter.BP_Interactable` null _asbp_third_person_character))

(event `INTERACTION`)

(fn `UserConstructionScript`)