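; Physics puzzle cube whose gravity the player flips by clicking it within reach.
; Clicks alternate GravityUP through a FlipFlop with a directional Niagara burst, and Tick applies upward acceleration to the mesh based on that state.
; RESPAWN plays a scale timeline, spawns a destroy effect, and replaces the actor with a new cube at its BeginPlay location, which plays its own scale animation.
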(event `self.ReceiveTick`
  (params (DeltaSeconds :type "Float (single-precision)"))
  (bind _sm_chamfercube (`self.SM_ChamferCube`))
  ;[0.15 0.15 0.15 0.5 50] EVENT TICK
  (`self.GravityUP`
    (:`then`
      (`PrimitiveComponent.AddForce` _sm_chamfercube (+ (0.0 0.0 10000.0) (`PrimitiveComponent.GetMass` _sm_chamfercube)) "None" true))
    (:`else`)))

(event `self.ReceiveBeginPlay`
  ;[0.15 0.15 0.15 0.5 50] BEGIN PLAY
  (set `self.Spawned AT` (`self.K2_GetActorLocation`)))

(event `self.ReceiveActorOnClicked`
  (params (ButtonPressed :type "Key Structure"))
  ;[0.15 0.15 0.15 0.5 50] ON CLICK CHANGE - LOOK HOW FAR THE PLAYER IS AND CHANGE GRAVITY
  (bind _asbp_third_person_character (cast `/Game/Blueprints/BP_ThirdPersonCharacter` (`GameplayStatics.GetPlayerCharacter` 0)))
  (bind _returnvalue (`KismetMathLibrary.VSize` (- (`SceneComponent.K2_GetComponentLocation` (`self.Box`)) (`self.K2_GetActorLocation` _asbp_third_person_character))))
  ;;[1 0.2912 0.001054 0.5] DEBUG DISTANCE
  (`KismetSystemLibrary.PrintString` (`KismetStringLibrary.Conv_DoubleToString` _returnvalue))
  (if (<= _returnvalue (`self.Max Reach Distance`))
    (`/Engine/EditorBlueprintResources/StandardMacros.FlipFlop`
      (:`A`
        (set `self.GravityUP` true)
        (`NiagaraFunctionLibrary.SpawnSystemAtLocation` "/Game/Graphics/Niagara_Systems/NS_Gravity.NS_Gravity" (+ (`SceneComponent.K2_GetComponentLocation` (`self.SM_ChamferCube`)) (0.0 0.0 100.0))))
      (:`B`
        (set `self.GravityUP` false)
        (`NiagaraFunctionLibrary.SpawnSystemAtLocation` "/Game/Graphics/Niagara_Systems/NS_Gravity.NS_Gravity" (+ (`SceneComponent.K2_GetComponentLocation` (`self.SM_ChamferCube`)) (0.0 0.0 -50.0)) (struct :`Roll` 180.0))))))

(event `RespawnAnim`
  ; play anim
  (bind (_direction _newtrack_0) (`Timeline|Timeline_0`)
    (:`Update`
      (`SceneComponent.SetRelativeScale3D` (`self.SM_ChamferCube`) (`KismetMathLibrary.Conv_DoubleToVector` _newtrack_0)))))

(event `RESPAWN`
  (bind _sm_chamfercube (`self.SM_ChamferCube`))
  ;[0.15 0.15 0.15 0.5 50] RESPAWN CUBE
  (set `self.GravityUP` false)
  (bind (_direction _newtrack_0) (`Timeline|Timeline`)
    (:`Update`
      (`SceneComponent.SetRelativeScale3D` _sm_chamfercube (`KismetMathLibrary.Conv_DoubleToVector` _newtrack_0)))
    (:`Finished`
      (`NiagaraFunctionLibrary.SpawnSystemAtLocation` "/Game/Graphics/Niagara_Systems/NS_CubeDestroy.NS_CubeDestroy" (`SceneComponent.K2_GetComponentLocation` _sm_chamfercube) (`SceneComponent.K2_GetComponentRotation` _sm_chamfercube))
      (`self.K2_DestroyActor`)
      (bind _returnvalue (`|SpawnActorFromClass` "BP_MasterCube_C" (`KismetMathLibrary.MakeTransform` (`self.Spawned AT`)) "Undefined" "MultiplyWithRoot" null null))
      (`self.RespawnAnim` _returnvalue))))

(fn `UserConstructionScript`)