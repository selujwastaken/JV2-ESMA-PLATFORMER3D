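; BP_MatDetector is a mass-detector trigger that consumes BP_MasterCube actors and opens a linked door once their accumulated mass reaches a goal.
; Mass labels face the player camera until the first cube removes them.
; Each overlapping cube snaps to an arrow, scales via timeline, then is destroyed with Niagara effects.
; Doors needing several detectors count completions before opening; otherwise one suffices, and insufficient mass shows a temporary tick.
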(event `self.ReceiveTick`
  (params (DeltaSeconds :type "Float (single-precision)"))
  (bind _character (`self.Character`))
  (bind _text_mass_current (`self.TEXT MASS CURRENT`))
  ; Comment
  (`/Engine/EditorBlueprintResources/StandardMacros.IsValid` _text_mass_current
    (:`Is Valid`
      (`TextRenderComponent.K2_SetText` _text_mass_current (`KismetTextLibrary.Conv_DoubleToText` (`self.Current Mass`) "HalfToEven"))
      (`/Engine/EditorBlueprintResources/StandardMacros.IsValid` _character
        (:`Is Valid`
          (`SceneComponent.K2_SetRelativeRotation` (`self.TEXT MASS GOAL`) (`KismetMathLibrary.FindLookAtRotation` (`self.K2_GetActorLocation`) (`SceneComponent.K2_GetComponentLocation` (`/Game/Blueprints/BP_ThirdPersonCharacter.FollowCamera` _character))) false false)
          (`SceneComponent.K2_SetRelativeRotation` (`self.TEXT MASS CURRENT`) (`KismetMathLibrary.FindLookAtRotation` (`self.K2_GetActorLocation`) (`SceneComponent.K2_GetComponentLocation` (`/Game/Blueprints/BP_ThirdPersonCharacter.FollowCamera` _character))) false false))))))

(event `self.ReceiveBeginPlay`
  ; Comment
  (`TextRenderComponent.K2_SetText` (`self.TEXT MASS GOAL`) (`KismetTextLibrary.Conv_DoubleToText` (`self.Mass Goal`) "HalfToEven"))
  (bind _returnvalue (`GameplayStatics.GetActorOfClass` "/Game/Blueprints/BP_ThirdPersonCharacter.BP_ThirdPersonCharacter_C"))
  (set `self.Character` _returnvalue))

(event `self.Box.OnComponentBeginOverlap`
  (params (OverlappedComponent :type "PrimitiveComponent Object Reference") (OtherActor :type "Actor Object Reference") (OtherComp :type "PrimitiveComponent Object Reference") (OtherBodyIndex :type Integer) (bFromSweep :type Boolean) (SweepResult :type "HitResult Structure (by ref)"))
  ; Comment
  (bind _asbp_master_cube (cast `/Game/Blueprints/BP_Cubes/BP_MasterCube` OtherActor))
  (set `self.As BP Key Cube` _asbp_master_cube)
  (set `self.Current Mass` (+ (`self.Current Mass`) (`PrimitiveComponent.GetMass` (`/Game/Blueprints/BP_Cubes/BP_MasterCube.SM_ChamferCube` _asbp_master_cube))))
  (`self.is goal acheaved`))

(event `is goal acheaved`
  (bind _doortoopen (`self.DoorToOpen`))
  (`self.destroy cube`)
  ; is goal achived
  (if (>= (`self.Current Mass`) (`self.Mass Goal`))
    (`/Game/Blueprints/BP_Door.need many ?` _doortoopen
      (:`then`
        (bind _output_get (set `/Game/Blueprints/BP_Door.TotalAchived` (+ (`/Game/Blueprints/BP_Door.TotalAchived` _doortoopen) 1.0) _doortoopen))
        (if (== _output_get (`/Game/Blueprints/BP_Door.totaltogetright` _doortoopen))
          (`/Engine/EditorBlueprintResources/StandardMacros.DoOnce` false
            (:`Completed`
              (`self.opendoor`)))
          (else
            (`PrimitiveComponent.SetMaterial` (`self.Mesh_Plane_ArrowCentre`) 0 "/Game/Graphics/Materials/M_Tick.M_Tick"))))
      (:`else`
        (`/Engine/EditorBlueprintResources/StandardMacros.DoOnce` false
          (:`Completed`
            (`self.opendoor`)))))
    (else
      (`self.correct`))))

(event `correct`
  (bind _mesh_plane_arrowcentre (`self.Mesh_Plane_ArrowCentre`))
  ; correct
  (`PrimitiveComponent.SetMaterial` _mesh_plane_arrowcentre 0 "/Game/Graphics/Materials/M_Tick.M_Tick")
  (`KismetSystemLibrary.Delay` 3.0)
  (`PrimitiveComponent.SetMaterial` _mesh_plane_arrowcentre 0 "/Game/Graphics/Materials/M_Anim_Arrow_center.M_Anim_Arrow_center"))

(event `destroy cube`
  (bind _arrow (`self.Arrow`))
  (bind _arrow_2 (`self.Arrow`))
  (bind _text_mass_goal (`self.TEXT MASS GOAL`))
  ; open the door
  (`/Engine/EditorBlueprintResources/StandardMacros.IsValid` (`self.As BP Key Cube`)
    (:`Is Valid`
      (`|ExecutionSequence`
        (:`then_0`
          (`PrimitiveComponent.SetSimulatePhysics` (`/Game/Blueprints/BP_Cubes/BP_MasterCube.SM_ChamferCube` (`self.As BP Key Cube`)) false))
        (:`then_1`
          (`SceneComponent.K2_SetWorldLocationAndRotation` (`/Game/Blueprints/BP_Cubes/BP_MasterCube.SM_ChamferCube` (`self.As BP Key Cube`)) (`SceneComponent.K2_GetComponentLocation` _arrow_2) (`SceneComponent.K2_GetComponentRotation` _arrow_2) false true))
        (:`then_2`
          (bind (_direction _newtrack_0) (`Timeline|Timeline` :!via `PlayFromStart`)
            (:`Update`
              (`SceneComponent.SetRelativeScale3D` (`/Game/Blueprints/BP_Cubes/BP_MasterCube.SM_ChamferCube` (`self.As BP Key Cube`)) (`KismetMathLibrary.Conv_DoubleToVector` _newtrack_0)))
            (:`Finished`
              (`self.K2_DestroyActor` (`self.As BP Key Cube`))
              (`NiagaraFunctionLibrary.SpawnSystemAtLocation` "/Game/Graphics/Niagara_Systems/NS_CubeDestroy.NS_CubeDestroy" (`SceneComponent.K2_GetComponentLocation` _arrow) (`SceneComponent.K2_GetComponentRotation` _arrow)))))
        (:`then_3`
          (`/Engine/EditorBlueprintResources/StandardMacros.IsValid` (`self.TEXT MASS CURRENT`)
            (:`Is Valid`
              (`/Engine/EditorBlueprintResources/StandardMacros.IsValid` _text_mass_goal
                (:`Is Valid`
                  (`ActorComponent.K2_DestroyComponent` _text_mass_goal)
                  (`ActorComponent.K2_DestroyComponent` (`self.TEXT MASS CURRENT`))
                  (`PrimitiveComponent.SetMaterial` (`self.Mesh_Plane_ArrowCentre`) 0 "/Game/Graphics/Materials/M_Tick.M_Tick"))))))))))

(event `opendoor`
  (`/Game/Blueprints/BP_Door.Open` (`self.DoorToOpen`)))

(fn `UserConstructionScript`)