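; BP_Door is a one-time opening door that can require a set count before it opens and can act as a checkpoint.
; Open fires the door directly, or, with NeedMultiple, only when the passed total equals TotalToGet.
; A DoOnce-guarded timeline then incrementally offsets the cube along Z and, for checkpoints, sets the player's CheckPoint to the arrow's location.
; The construction script shows requirement text only for multiple-item doors.
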(event `Open`
  (params (`Total Achived` :type Integer))
  (`self.need Multiple ?`
    (:`then`
      (`KismetSystemLibrary.PrintString` (`KismetStringLibrary.Conv_IntToString` `Total Achived`) true true (struct :`G` 0.66 :`B` 1.0 :`A` 1.0) 20.0)
      (if (== `Total Achived` (`self.total to get`))
        (`/Engine/EditorBlueprintResources/StandardMacros.DoOnce` false :!label _label
          (:`Completed`
            (bind (_direction _newtrack_0) (`Timeline|door`)
              (:`Update`
                (`SceneComponent.K2_AddLocalOffset` (`self.Cube`) (`KismetMathLibrary.MakeVector` 0.0 0.0 (* _newtrack_0 10.0)) false false)
                (`self.Is A CheckPoint`
                  (:`then`
                    (bind _asbp_third_person_character (cast `/Game/Blueprints/BP_ThirdPersonCharacter` (`GameplayStatics.GetPlayerCharacter` 0)))
                    (set `/Game/Blueprints/BP_ThirdPersonCharacter.CheckPoint` (`SceneComponent.K2_GetComponentLocation` (`self.Arrow`)) _asbp_third_person_character))
                  (:`else`))))))))
    (:`else`
      (goto _label))))

(fn `UserConstructionScript`
  (bind _number_left (`self.NUMBER LEFT`))
  (`self.need Multiple ?`
    (:`then`
      (`SceneComponent.SetVisibility` _number_left true false)
      (`SceneComponent.SetVisibility` (`self.You Have`) true false)
      (`TextRenderComponent.K2_SetText` (`self.NUMBER LEFT`) (`KismetTextLibrary.Conv_StringToText` (`KismetStringLibrary.Concat_StrStr` "YOU NEED : " (`KismetStringLibrary.Conv_IntToString` (`self.total to get`)) " LEFT"))))
    (:`else`
      (`SceneComponent.SetVisibility` _number_left false false)
      (`SceneComponent.SetVisibility` (`self.You Have`) false false))))