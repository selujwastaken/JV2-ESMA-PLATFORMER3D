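; BP_Moving_Platform is an actor that moves between its starting location and a point offset from it.
; On BeginPlay it stores its location as PointA, then builds PointB from per-axis X, Y and Z values scaled by 100, each gated by a Use check.
; The MovingPatern timeline then drives a vector lerp between the two points, setting the actor location each update without sweep.
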(event `self.ReceiveBeginPlay`
  (set `self.Point A` (`self.K2_GetActorLocation`))
  (`|ExecutionSequence`
    (:`then_0`
      (`self.Use X`
        (:`then`
          (bind _returnvalue (`KismetMathLibrary.MakeVector` (* (`self.Value_X`) 100.0))))
        (:`else`)))
    (:`then_1`
      (`self.Use Y`
        (:`then`
          (bind _returnvalue_2 (`KismetMathLibrary.MakeVector` 0.0 (* (`self.Value_Y`) 100.0))))
        (:`else`)))
    (:`then_2`
      (`self.Use Z`
        (:`then`
          (bind _returnvalue_3 (`KismetMathLibrary.MakeVector` 0.0 0.0 (* (`self.Value_Z`) 100.0))))
        (:`else`)))
    (:`then_3`
      (set `self.Point B` (+ (`self.Point A`) _returnvalue _returnvalue_2 _returnvalue_3))
      (bind (_direction _newtrack_0) (`Timeline|moving patern`)
        (:`Update`
          (`self.K2_SetActorLocation` (`KismetMathLibrary.VLerp` (`self.Point A`) (`self.Point B`) _newtrack_0)))))))

(fn `UserConstructionScript`)