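; BP_Master_Asteroid is an asteroid actor that randomizes its size and launches itself when play begins.
; About one in ten gets a much larger scale, with each axis randomized independently for uneven shapes.
; A velocity-change impulse then multiplies the normalized direction to BP_ThirdPersonCharacter component-wise by a random unit vector, so it is not truly aimed at the player.
; Without a valid character, the impulse is fully random per axis.
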(event `self.ReceiveBeginPlay`
  (bind _returnvalue (`KismetMathLibrary.RandomFloatInRange` 0.5 3.0))
  (bind _asteroid_mesh (`self.Asteroid_Mesh`))
  (bind _returnvalue_2 (* _returnvalue (`KismetMathLibrary.RandomFloatInRange` 5.0 10.0)))
  (if (> (`KismetMathLibrary.RandomFloatInRange` 0.0 1.0) 0.9)
    (`SceneComponent.SetRelativeScale3D` (`self.Asteroid_Mesh`) (`KismetMathLibrary.MakeVector` _returnvalue_2 _returnvalue_2 _returnvalue_2))
    (else
      (`SceneComponent.SetRelativeScale3D` (`self.Asteroid_Mesh`) (`KismetMathLibrary.MakeVector` _returnvalue _returnvalue _returnvalue))))
  (bind _returnvalue_3 (`GameplayStatics.GetActorOfClass` "/Game/Blueprints/BP_ThirdPersonCharacter.BP_ThirdPersonCharacter_C"))
  (`/Engine/EditorBlueprintResources/StandardMacros.IsValid` _returnvalue_3
    (:`Is Valid`
      (`PrimitiveComponent.AddImpulse` _asteroid_mesh (* (* (`KismetMathLibrary.Normal` (- (`self.K2_GetActorLocation` _returnvalue_3) (`self.K2_GetActorLocation`))) (* (`KismetMathLibrary.RandomUnitVector`) 50.0)) (`KismetMathLibrary.RandomFloatInRange` 20.0 60.0)) "None" true))
    (:`Is Not Valid`
      (`PrimitiveComponent.AddImpulse` _asteroid_mesh (`KismetMathLibrary.MakeVector` (`KismetMathLibrary.RandomFloatInRange` -1000.0 1000.0) (`KismetMathLibrary.RandomFloatInRange` -1000.0 1000.0) (`KismetMathLibrary.RandomFloatInRange` -1000.0 1000.0)) "None" true))))

(fn `UserConstructionScript`)