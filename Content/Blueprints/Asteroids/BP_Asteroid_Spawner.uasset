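; BP_Asteroid_Spawner is an actor that maintains a field of randomly chosen asteroids around its location.
; On BeginPlay it spawns SpawnHowMuch asteroids in random directions between MinRadius and MaxRadius, each with random rotation.
; A looping five-second timer reuses that spawn logic to add more.
; Any BP_Master_Asteroid leaving the Sphere overlap is destroyed and replaced through the same logic, recycling the field.
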(event `self.ReceiveBeginPlay`
  (bind _returnvalue (`KismetMathLibrary.RandomFloatInRange` 0.0 360.0))
  (bind _returnvalue_2 (`GameplayStatics.GetActorOfClass` "/Game/Blueprints/Actors/Pawn/BP_ThirdPersonCharacter.BP_ThirdPersonCharacter_C"))
  (set `self.PlayerCharacter` _returnvalue_2)
  (for _ (range 1 (+ (`self.Spawn_How_Much`) 1))
    (`|SpawnActorFromClass` (`KismetArrayLibrary.Array_Random` (`self.All_Asteroids`)) (`KismetMathLibrary.MakeTransform` (+ (`self.K2_GetActorLocation`) (* (`KismetMathLibrary.Normal` (`KismetMathLibrary.MakeVector` (`KismetMathLibrary.RandomFloatInRange` -1.0 1.0) (`KismetMathLibrary.RandomFloatInRange` -1.0 1.0) (`KismetMathLibrary.RandomFloatInRange` -1.0 1.0))) (`KismetMathLibrary.RandomFloatInRange` (`self.Min_Radius`) (`self.Max_Radius`)))) (`KismetMathLibrary.MakeRotator` _returnvalue _returnvalue _returnvalue)) "Undefined" "MultiplyWithRoot" null null :!label _label))
  (`KismetSystemLibrary.K2_SetTimerDelegate` (delegate `Spawn Asteroid`) 5.0 true))

(event `Spawn Asteroid`
  (goto _label))

(event `self.Sphere.OnComponentEndOverlap`
  (params (OverlappedComponent :type "PrimitiveComponent Object Reference") (OtherActor :type "Actor Object Reference") (OtherComp :type "PrimitiveComponent Object Reference") (OtherBodyIndex :type Integer))
  (bind _asbp_master_asteroid (cast `/Game/Blueprints/Asteroids/BP_Master_Asteroid` OtherActor))
  (`self.K2_DestroyActor` _asbp_master_asteroid)
  (goto _label))

(fn `UserConstructionScript`)