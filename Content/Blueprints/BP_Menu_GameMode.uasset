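; Game mode for the menu that opens either the main menu or a first-time key screen.
; On BeginPlay it disables player controller input and switches the view to a CameraActor found in the level.
; It checks KeyMappingCompleted on BP_GameInstance to choose between ShowMainMenu and a one-time WBP_Keys widget, which also sets that flag.
; ShowMainMenu clears all widgets and adds WBP_ScreenMenu to the viewport.
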(event `self.ReceiveBeginPlay`
  (bind _returnvalue (`GameplayStatics.GetPlayerController` 0))
  (`self.DisableInput` _returnvalue _returnvalue)
  (bind _returnvalue_2 (`GameplayStatics.GetActorOfClass` "/Script/Engine.CameraActor"))
  (`PlayerController.SetViewTargetWithBlend` _returnvalue _returnvalue_2 0.0 "VTBlend_Linear" 0.0 false)
  (bind _asbp_game_instance (cast `/Game/Blueprints/BP_GameInstance` (`GameplayStatics.GetGameInstance`)))
  (`/Game/Blueprints/BP_GameInstance.KeyMappingCompleted` _asbp_game_instance
    (:`then`
      (`self.Show Main Menu`))
    (:`else`
      (`/Engine/EditorBlueprintResources/StandardMacros.DoOnce` false
        (:`Completed`
          (bind _returnvalue_3 (`|CreateWidget` "/Game/Widgets/WBP_Keys.WBP_Keys_C"))
          (`UserWidget.AddToViewport` _returnvalue_3 0)
          (set `/Game/Blueprints/BP_GameInstance.KeyMappingCompleted` true _asbp_game_instance))))))

(event `Show Main Menu`
  (`WidgetLayoutLibrary.RemoveAllWidgets`)
  (bind _returnvalue (`|CreateWidget` "/Game/Widgets/WBP_ScreenMenu.WBP_ScreenMenu_C"))
  (`UserWidget.AddToViewport` _returnvalue 0))

(fn `UserConstructionScript`)